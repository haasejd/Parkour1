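; BP_Parkour_Fence is an AdventureKit parkour zone for fences, with two usable sides.
; It returns forward and right vectors for whichever side a queried world location is on.
; Each getter transforms the location into actor space and negates the actor's vector when local X is negative.
; The construction script is empty, and the file contains no traversal logic of its own.
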(fn ConstructionScript)

(fn GetClosestZoneRightVector
  (params (ToWorldLocation :type Vector%20%28by%20ref%29))
  (bind _returnvalue (Transformation|GetActorRightVector))
  ;[0.1 0.1 0.1] The zone has two sides and the right vector is different depening on which side the query location is
  (if (>= (.x (Math|Transform|InverseTransformLocation (Transformation|GetActorTransform) ToWorldLocation)) 0.0)
    (return _returnvalue)
    (else
      (return (* _returnvalue -1.0)))))

(fn GetClosestZoneForwardVector
  (params (ToWorldLocation :type Vector%20%28by%20ref%29))
  (bind _returnvalue (Transformation|GetActorForwardVector))
  ;[0.1 0.1 0.1] The zone has two sides and the forward vector is different depening on which side the query location is
  (if (>= (.x (Math|Transform|InverseTransformLocation (Transformation|GetActorTransform) ToWorldLocation)) 0.0)
    (return _returnvalue)
    (else
      (return (* _returnvalue -1.0)))))