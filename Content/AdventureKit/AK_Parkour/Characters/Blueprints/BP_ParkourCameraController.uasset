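; Camera controller for the parkour character that restricts camera rotation during falling rolls and slides.
; After the parent Tick, it checks the owner for the falling roll montage or the sliding state.
; While either is active, it disables controller desired rotation on the advanced movement component and pawn control rotation on the first configured camera.
; It also turns off that configuration's pitch, yaw and roll clamps to prevent controller overrides.
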(event EventTick
  (params (DeltaSeconds :type Float%20%28single-precision%29))
  (bind _cameraconfigurations (Variables|Default|GetCameraConfigurations))
  (bind _item (Utilities|Array|Get(acopy) _cameraconfigurations))
  (|CallParentFunction DeltaSeconds)
  ;[0.1 0.1 0.1] Restrict the camera rotation based on the floor rolling montage and during sliding
  (bind _asbp_parkour_character (Utilities|Casting|CastToBP_ParkourCharacter (Components|GetOwner)))
  (bind _returnvalue (Animation|GetCurrentMontage _asbp_parkour_character :!class /Script/Engine.Character))
  (Variables|/Script/Engine.CharacterMovementComponent|SetbUseControllerDesiredRotation (Class|AdvKitCharacter|GetAdvMovementComponent _asbp_parkour_character) (not (or (== _returnvalue "/Game/AdventureKit/AK_Parkour/Characters/Montages/AM_Parkour_FallingRoll.AM_Parkour_FallingRoll") (Variables|/Game/AdventureKit/AK_Parkour/Characters/Blueprints/BP_ParkourCharacter.BP_ParkourCharacter_C|GetIs%20Sliding _asbp_parkour_character))))
  ;[0.1 0.1 0.1] Prevent camera from turning
  (Variables|/Script/Engine.CameraComponent|SetbUsePawnControlRotation (.Camera (Utilities|Struct|BreakCameraConfig _item)) (not (or (== _returnvalue "/Game/AdventureKit/AK_Parkour/Characters/Montages/AM_Parkour_FallingRoll.AM_Parkour_FallingRoll") (Variables|/Game/AdventureKit/AK_Parkour/Characters/Blueprints/BP_ParkourCharacter.BP_ParkourCharacter_C|GetIs%20Sliding _asbp_parkour_character))))
  ;[0.1 0.1 0.1] Prevent camera controller overriding
  (bind _structout (Utilities|Struct|SetmembersinCameraConfig _item (not (or (== _returnvalue "/Game/AdventureKit/AK_Parkour/Characters/Montages/AM_Parkour_FallingRoll.AM_Parkour_FallingRoll") (Variables|/Game/AdventureKit/AK_Parkour/Characters/Blueprints/BP_ParkourCharacter.BP_ParkourCharacter_C|GetIs%20Sliding _asbp_parkour_character))) (not (or (== _returnvalue "/Game/AdventureKit/AK_Parkour/Characters/Montages/AM_Parkour_FallingRoll.AM_Parkour_FallingRoll") (Variables|/Game/AdventureKit/AK_Parkour/Characters/Blueprints/BP_ParkourCharacter.BP_ParkourCharacter_C|GetIs%20Sliding _asbp_parkour_character))) (not (or (== _returnvalue "/Game/AdventureKit/AK_Parkour/Characters/Montages/AM_Parkour_FallingRoll.AM_Parkour_FallingRoll") (Variables|/Game/AdventureKit/AK_Parkour/Characters/Blueprints/BP_ParkourCharacter.BP_ParkourCharacter_C|GetIs%20Sliding _asbp_parkour_character)))))
  (Utilities|Array|SetArrayElem (Variables|Default|GetCameraConfigurations) 0 _structout))