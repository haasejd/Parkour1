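; Transition builder module that generates step-up and step-down movement transitions within a single BP_LadderZone.
; It only accepts ladder zones with ClimbingLadder physics and connects each zone to itself.
; It loops over step pairs, skipping those near both ends, and creates opposing transition points two step heights apart.
; Endpoints are transformed from ladder space and constrained to the zone using the character's half extent, keeping the ladder's movement mode.
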(fn CreateTransitionBetween
  (params (ForCharacterClass :type Adv%20Kit%20Character%20Class%20Reference) (SourceZone :type Adv%20Kit%20Zone%20Object%20Reference) (TargetZone :type Adv%20Kit%20Zone%20Object%20Reference))
  ;[0.1 0.1 0.1] Check if transitions can be created
  (LocalVariables|SetCharacter%20Class ForCharacterClass)
  (if (== SourceZone TargetZone)
    (bind _asbp_ladder_zone (Utilities|Casting|CastToBP_LadderZone SourceZone)
      (:then
        (Utilities|FlowControl|Sequence
          (:then_0
            ;[0.1 0.1 0.1] Configuration
            (LocalVariables|SetCurrent%20Ladder _asbp_ladder_zone)
            (LocalVariables|SetStep%20Height (Variables|/Game/ParkourBlueprints/BP_LadderZone.BP_LadderZone_C|GetStep%20Height _asbp_ladder_zone))
            (LocalVariables|SetStep%20Count (Variables|/Game/ParkourBlueprints/BP_LadderZone.BP_LadderZone_C|GetStep%20Count _asbp_ladder_zone)))
          (:then_1
            ;[0.1 0.1 0.1] Create transitions to step up and down
            ;;[0.1 0.1 0.1] Iterate over steps (minus first and last)
            (for _index (range (Class|KismetSystemLibrary|MakeLiteralInteger 2) (- (/ (LocalVariables|GetStep%20Count) 2) 2))
              (bind _returnvalue (Class|AdvKitZone|GetCustomPhysics (LocalVariables|GetCurrent%20Ladder)))
              (bind _returnvalue_2 (Class|AdvKitZone|GetPhysics (LocalVariables|GetCurrent%20Ladder)))
              (Utilities|FlowControl|Sequence
                (:then_0
                  ;;[0.1 0.1 0.1] Create Step down
                  (Class|AdvKitTransitionBuilderModule|CreateTransitionPoint self (Utilities|String|ToString(Text) (Utilities|Text|FormatText "StepDown{number}" (Utilities|Text|ToText(Integer) _index))) (LocalVariables|GetCurrent%20Ladder) (Class|AdvKitZone|ConstrainPositiontoZone (LocalVariables|GetCurrent%20Ladder) (Math|Transform|TransformLocation (Transformation|GetActorTransform (LocalVariables|GetCurrent%20Ladder)) (Math|Vector|MakeVector 0.0 0.0 (* (* (+ _index 1) 2) (LocalVariables|GetStep%20Height)))) (Class|AdvKitTransitionBuilderModule|GetCharacterHalfExtent (LocalVariables|GetCharacter%20Class) (LocalVariables|GetCurrent%20Ladder)) (Transformation|GetActorRotation (LocalVariables|GetCurrent%20Ladder))) (Class|AdvKitZone|ConstrainPositiontoZone (LocalVariables|GetCurrent%20Ladder) (Math|Transform|TransformLocation (Transformation|GetActorTransform (LocalVariables|GetCurrent%20Ladder)) (Math|Vector|MakeVector 0.0 0.0 (* (* _index 2) (LocalVariables|GetStep%20Height)))) (Class|AdvKitTransitionBuilderModule|GetCharacterHalfExtent (LocalVariables|GetCharacter%20Class) (LocalVariables|GetCurrent%20Ladder)) (Transformation|GetActorRotation (LocalVariables|GetCurrent%20Ladder))) (LocalVariables|GetCharacter%20Class) _returnvalue_2 (LocalVariables|GetCurrent%20Ladder) _returnvalue))
                (:then_1
                  ;;[0.1 0.1 0.1] Create Step up
                  (Class|AdvKitTransitionBuilderModule|CreateTransitionPoint self (Utilities|String|ToString(Text) (Utilities|Text|FormatText "StepUp{number}" (Utilities|Text|ToText(Integer) _index))) (LocalVariables|GetCurrent%20Ladder) (Class|AdvKitZone|ConstrainPositiontoZone (LocalVariables|GetCurrent%20Ladder) (Math|Transform|TransformLocation (Transformation|GetActorTransform (LocalVariables|GetCurrent%20Ladder)) (Math|Vector|MakeVector 0.0 0.0 (* (* _index 2) (LocalVariables|GetStep%20Height)))) (Class|AdvKitTransitionBuilderModule|GetCharacterHalfExtent (LocalVariables|GetCharacter%20Class) (LocalVariables|GetCurrent%20Ladder)) (Transformation|GetActorRotation (LocalVariables|GetCurrent%20Ladder))) (Class|AdvKitZone|ConstrainPositiontoZone (LocalVariables|GetCurrent%20Ladder) (Math|Transform|TransformLocation (Transformation|GetActorTransform (LocalVariables|GetCurrent%20Ladder)) (Math|Vector|MakeVector 0.0 0.0 (* (* (+ _index 1) 2) (LocalVariables|GetStep%20Height)))) (Class|AdvKitTransitionBuilderModule|GetCharacterHalfExtent (LocalVariables|GetCharacter%20Class) (LocalVariables|GetCurrent%20Ladder)) (Transformation|GetActorRotation (LocalVariables|GetCurrent%20Ladder))) (LocalVariables|GetCharacter%20Class) _returnvalue_2 (LocalVariables|GetCurrent%20Ladder) _returnvalue)))))
          (:then_2
            ;[0.1 0.1 0.1] Done
            (return true))))
      (:CastFailed
        (return false)))
    (else
      (return false))))

(fn CanCreateTransitionsfor
  (params (ForCharacterClass :type Adv%20Kit%20Character%20Class%20Reference) (ForZone :type Adv%20Kit%20Zone%20Object%20Reference))
  ;[0.1 0.1 0.1] Can only create steps for ladder zones that have ladder physics
  (bind _asbp_ladder_zone (Utilities|Casting|CastToBP_LadderZone ForZone)
    (:then
      (bind _returnvalue (Class|AdvKitZone|HasPhysics _asbp_ladder_zone "ClimbingLadder"))
      (return _returnvalue))
    (:CastFailed
      (return false))))

(fn CreateTransitionsfor
  (params (ForCharacterClass :type Adv%20Kit%20Character%20Class%20Reference) (ForZone :type Adv%20Kit%20Zone%20Object%20Reference))
  ;[0.1 0.1 0.1] Creates transitions inside the same zone
  (CallFunction|CreateTransitionBetween ForCharacterClass ForZone ForZone)
  (return))