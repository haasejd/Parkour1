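; BP_LedgeZone_Static is a parkour ledge zone that builds itself in the Construction Script from an editable ZoneStart point.
; It derives a symmetric ZoneEnd, width and thickness from that point to size the Overlap box.
; Optional corner flags then widen and offset a scaled, collision-free ledge mesh with assigned materials.
; A RegenerateTransitions flag triggers GenerateTransitions, resetting afterward unless AlwaysRegenerateTransitions is set.
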(fn ConstructionScript
  ;[0.1 0.1 0.1] Sort ledge variables
  (Variables|Default|SetZoneEnd (Math|Vector|MakeVector (.Z (Math|Vector|BreakVector (Variables|Default|GetZoneStart))) (* (.Y (Math|Vector|BreakVector (Variables|Default|GetZoneStart))) -1.0) (.Z (Math|Vector|BreakVector (Variables|Default|GetZoneStart)))))
  (Variables|Default|SetZoneStart (Math|Vector|MakeVector (.Z (Math|Vector|BreakVector (Variables|Default|GetZoneStart))) (.Y (Math|Vector|BreakVector (Variables|Default|GetZoneStart))) (.Z (Math|Vector|BreakVector (Variables|Default|GetZoneStart)))))
  (LocalVariables|SetLedgeWidth (Math|Float|Absolute(Float) (.Y (Math|Vector|BreakVector (Variables|Default|GetZoneStart)))))
  (Variables|Ledge|SetLedgeThickness (.X (Math|Vector|BreakVector (Variables|Default|GetZoneStart))))
  ;[0.1 0.1 0.1] Configure and place box component
  (Components|Box|SetBoxExtent (Variables|Default|GetOverlap) (Math|Vector|MakeVector (Variables|Ledge|GetLedgeThickness) (LocalVariables|GetLedgeWidth) (Variables|Ledge|GetLedgeThickness)) true)
  ;[0.1 0.1 0.1] Corner Additions
  (Utilities|FlowControl|Sequence
    (:then_0
      (if (Variables|Ledge|GetCorner%20At%20End)
        (LocalVariables|SetStart%20Offset (Math|Vector|MakeVector 0.0 (* (Variables|Ledge|GetLedgeThickness) 1.0) 0.0))
        (LocalVariables|SetLedgeWidth (+ (LocalVariables|GetLedgeWidth) (Variables|Ledge|GetLedgeThickness)) :!label _label)))
    (:then_1
      (if (Variables|Ledge|GetCorner%20At%20Start)
        (LocalVariables|SetStart%20Offset (Math|Vector|MakeVector 0.0 (+ (* (Variables|Ledge|GetLedgeThickness) -1.0) (.y (LocalVariables|GetStart%20Offset))) 0.0))
        (goto _label)))
    (:then_2
      ;[0.1 0.1 0.1] Create and place ledge mesh
      (Utilities|IsValid (Variables|Ledge|GetLedgeMesh)
        (:Is%20Valid
          (bind _returnvalue (AddComponent|AddStaticMeshComponent false))
          (bind _output_get (Variables|Default|SetLedge _returnvalue))
          (bind _returnvalue_2 (Components|StaticMesh|SetStaticMesh _output_get (Variables|Ledge|GetLedgeMesh)))
          (if _returnvalue_2
            (for (_array_element _array_index) (Variables|Ledge|GetLedgeMaterials)
              (Rendering|Material|SetMaterial (Variables|Default|GetLedge) _array_index _array_element))
            (Transformation|SetRelativeScale3D (Variables|Default|GetLedge) (* (Math|Vector|MakeVector (Variables|Ledge|GetLedgeThickness) (LocalVariables|GetLedgeWidth) (Variables|Ledge|GetLedgeThickness)) 0.02))
            (Transformation|SetRelativeLocation (Variables|Default|GetLedge) (+ (Math|Vector|MakeVector 0.0 0.0 (* (Variables|Ledge|GetLedgeThickness) -1.0)) "0, 0, 0" (LocalVariables|GetStart%20Offset)) false false)
            (Collision|SetCollisionEnabled (Variables|Default|GetLedge) "NoCollision")))))
    (:then_3
      ;[0.1 0.1 0.1] Create Transitions
      (if (Variables|Ledge|GetRegenerate%20Transitions)
        (Utilities|FlowControl|Sequence
          (:then_0
            (if (not (Variables|Ledge|GetAlways%20Regenerate%20Transitions))
              (Variables|Ledge|SetRegenerate%20Transitions false)))
          (:then_1
            (Class|AdvKitZone|GenerateTransitions true)))))))