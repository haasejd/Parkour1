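; BP_ZiplineZone is a parkour zipline actor that defines a capsule zone and a visible rope between a start and an end point.
; The construction script rotates, centers and sizes the capsule to span ZoneStart to ZoneEnd, so the zone follows the edited points.
; On BeginPlay, InitRope sets the rope particle beam's target to ZoneEnd in world space and applies RopeColor.
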(event EventBeginPlay
  (CallFunction|InitRope))

(fn ConstructionScript
  ;[1 1 1] Align capsule to zone extent
  (Transformation|SetRelativeRotation (Variables|Default|GetCapsule) (Math|Rotator|FindLookatRotation (Variables|Default|GetZoneStart) (Variables|Default|GetZoneEnd)) false false)
  (Transformation|AddLocalRotation (Variables|Default|GetCapsule) "90.000000,0.000000,0.000000" false false)
  (Transformation|SetRelativeLocation (Variables|Default|GetCapsule) (Math|Vector|Lerp(Vector) (Variables|Default|GetZoneStart) (Variables|Default|GetZoneEnd) 0.5) false false)
  (Components|Capsule|SetCapsuleHalfHeight (Variables|Default|GetCapsule) (* (Math|Vector|VectorLength (- (Variables|Default|GetZoneStart) (Variables|Default|GetZoneEnd))) 0.5) true))

(fn InitRope
  (bind _rope (Variables|Default|GetRope))
  ;[0.1 0.1 0.1] Set rope beam point
  (Class|ParticleSystemComponent|SetBeamTargetPoint _rope 0 (Math|Transform|TransformLocation (Transformation|GetActorTransform) (Variables|Default|GetZoneEnd)))
  ;[0.1 0.1 0.1] Set rope color
  (Effects|Components|ParticleSystem|SetColorParameter _rope "Color" (Variables|Default|GetRope%20Color)))